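; Raycast car Blueprint that sets up four-wheel suspension ground detection; it applies no forces yet.
; BeginPlay caches the four TopLink components, derives each ray length from suspension and wheel radius, and starts lengths at rest.
; Each Tick traces down each link's local up axis with debug drawing, storing contacts and hits.
; Airborne wheels get full-extension length; the grounded-length calculation is present but unconnected.
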(event `self.ReceiveBeginPlay`
  (`self.StoreComponentToArray`)
  (`self.rayCast_INI`)
  (`self.Suspension_INI`))

(event `self.ReceiveTick`
  (params (DeltaSeconds :type "Float (single-precision)"))
  (set `self.DeltaTime` DeltaSeconds)
  (`self.rayCast_lineTrace`)
  (for _index (range 4)
    (if (not (`|GetArrayItem` (`self.WheelContact`) _index))
      (bind (_rest_length _travel) (break `/Game/Blueprints/SuspensionStruct` (`|GetArrayItem` (`self.Suspension`) _index)))
      (`KismetArrayLibrary.Array_Set` (`self.Length`) _index (+ _rest_length _travel)))))

(fn `rayCast_INI`
  (for _index (range 4)
    (bind (_rest_length _travel) (break `/Game/Blueprints/SuspensionStruct` (`|GetArrayItem` (`self.Suspension`) _index)))
    (`KismetArrayLibrary.Array_Set` (`self.RayLength`) _index (+ (+ _rest_length _travel) (`.Radius_2_699D6A2D4A8E9C41C2D6FE989E7581CF` (break `/Game/Blueprints/WheelStruct` (`|GetArrayItem` (`self.Wheel`) _index)))))))

(fn `rayCast_lineTrace`
  (for _index (range 4)
    (bind _output (`|GetArrayItem` (`self.TopLinkComponent`) _index))
    (bind _returnvalue (`SceneComponent.K2_GetComponentLocation` _output))
    (bind (_outhit _returnvalue_2) (`KismetSystemLibrary.LineTraceSingle` :`Start` _returnvalue :`End` (- _returnvalue (* (`SceneComponent.GetUpVector` _output) (`|GetArrayItem` (`self.RayLength`) _index))) :`TraceChannel` "TraceTypeQuery1" :`DrawDebugType` "ForDuration" :`TraceColor` (struct :`G` 0.040663 :`B` 1.0 :`A` 1.0) :`TraceHitColor` (struct :`G` 1.0 :`B` 0.421747 :`A` 1.0) :`DrawTime` 1.0))
    (`KismetArrayLibrary.Array_Set` (`self.WheelContact`) _index _returnvalue_2)
    (if _returnvalue_2
      (`KismetArrayLibrary.Array_Set` (`self.HitRes`) _index _outhit)
      (`KismetSystemLibrary.PrintString` (`KismetStringLibrary.Conv_BoolToString` _returnvalue_2) true false (struct :`R` 0.114604 :`G` 1.0 :`A` 1.0) 0.0))))

(fn `StoreComponentToArray`
  (for _index (range 4)
    (`KismetArrayLibrary.Array_Set` (`self.TopLinkComponent`) _index (select `int` _index :`0` (`self.TopLink_FR`) :`1` (`self.TopLink_RR`) :`2` (`self.TopLink_RL`) :`3` (`self.TopLink_FL`)))))

(fn `Suspension_INI`
  (for _index (range 4)
    (`KismetArrayLibrary.Array_Set` (`self.Length`) _index (`.rest_length_3_C1B3A0414ABA35C19F70A3868A705A9E` (break `/Game/Blueprints/SuspensionStruct` (`|GetArrayItem` (`self.Suspension`) _index))))))

(fn `UserConstructionScript`)